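; BP_PlayerControllerCustom is a player controller that switches the local player between gameplay and menu input.
; EnableGameInput swaps the Enhanced Input context from IM_Menu to IM_Default, sets game-only input, hides the cursor and focuses the game viewport.
; EnableMenuInput swaps to IM_Menu with forced immediate updates, sets game-and-UI input and shows the cursor.
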(event `Enable Game Input`
  (bind _returnvalue (subsystem `EnhancedInputLocalPlayerSubsystem`))
  (`EnhancedInputSubsystemInterface.RemoveMappingContext` _returnvalue "/Game/Input/IM_Menu.IM_Menu" (struct))
  (`EnhancedInputSubsystemInterface.AddMappingContext` _returnvalue "/Game/Input/IM_Default.IM_Default" 0 (struct))
  (`WidgetBlueprintLibrary.SetInputMode_GameOnly` self)
  (set `self.bShowMouseCursor` false)
  (`WidgetBlueprintLibrary.SetFocusToGameViewport`))

(event `Enable Menu Input`
  (bind _returnvalue (subsystem `EnhancedInputLocalPlayerSubsystem`))
  (`EnhancedInputSubsystemInterface.RemoveMappingContext` _returnvalue "/Game/Input/IM_Default.IM_Default" (make `ModifyContextOptions` true true))
  (`EnhancedInputSubsystemInterface.AddMappingContext` _returnvalue "/Game/Input/IM_Menu.IM_Menu" 0 (make `ModifyContextOptions` true true))
  (`WidgetBlueprintLibrary.SetInputMode_GameAndUIEx` self null)
  (set `self.bShowMouseCursor` true))

(fn `UserConstructionScript`)