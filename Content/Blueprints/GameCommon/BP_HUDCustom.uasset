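; Custom HUD Blueprint that owns the game's menu widget and toggles it on and off.
; BeginPlay creates and stores a WBP_Menu instance and caches the player's BP_PlayerControllerCustom.
; ToggleMune checks the widget's visibility, calls its Show or Hide, then has the controller switch to menu or game input.
; The toggle re-casts player controller 0 each time instead of using the cached reference.
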(event `self.ReceiveBeginPlay`
  (bind _returnvalue (`|CreateWidget` "/CommonInterface/Widget/WBP_Menu.WBP_Menu_C"))
  (set `self.Menu Widget` _returnvalue)
  (bind _asbp_player_controller_custom (cast `/Game/Blueprints/GameCommon/BP_PlayerControllerCustom` (`GameplayStatics.GetPlayerController` 0)))
  (set `self.Player Controller` _asbp_player_controller_custom))

(event `Toggle Mune`
  (if (`self.Is Menu Visible`)
    (bind _menu_widget (`self.Menu Widget`)
      (:`then`
        (`/CommonInterface/Widget/WBP_Menu.Hide` _menu_widget)
        (bind _asbp_player_controller_custom (cast `/Game/Blueprints/GameCommon/BP_PlayerControllerCustom` (`GameplayStatics.GetPlayerController` 0)))
        (`/Game/Blueprints/GameCommon/BP_PlayerControllerCustom.Enable Game Input` _asbp_player_controller_custom))
      (:`else`))
    (else
      (bind _menu_widget_2 (`self.Menu Widget`)
        (:`then`
          (`/CommonInterface/Widget/WBP_Menu.Show` _menu_widget_2)
          (bind _asbp_player_controller_custom_2 (cast `/Game/Blueprints/GameCommon/BP_PlayerControllerCustom` (`GameplayStatics.GetPlayerController` 0)))
          (`/Game/Blueprints/GameCommon/BP_PlayerControllerCustom.Enable Menu Input` _asbp_player_controller_custom_2))
        (:`else`)))))

(fn `Is Menu Visible`
  (returns (`Is Visible` :type Boolean))
  (return (`Widget.IsVisible` (`self.Menu Widget`))))

(fn `UserConstructionScript`)